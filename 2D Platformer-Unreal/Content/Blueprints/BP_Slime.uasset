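; BP_Slime is a 2D flipbook slime enemy that patrols by moving along its forward vector every tick.
; It reverses by rotating the actor half a turn when EdgeDetector ends an overlap or Box begins one, with no filter on the other actor.
; PlayDead, not called within this Blueprint, sets the dead flag, swaps to the death flipbook, plays a hit sound and destroys the actor after a short delay.
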(event `self.ReceiveTick`
  (params (DeltaSeconds :type "Float (single-precision)"))
  (`self.AddMovementInput` (`self.GetActorForwardVector`)))

(event `TurnActor`
  (`self.K2_SetActorRotation` (`KismetMathLibrary.ComposeRotators` (`self.K2_GetActorRotation`) (struct :`Yaw` 180.0))))

(event `self.EdgeDetector.OnComponentEndOverlap`
  (params (OverlappedComponent :type "PrimitiveComponent Object Reference") (OtherActor :type "Actor Object Reference") (OtherComp :type "PrimitiveComponent Object Reference") (OtherBodyIndex :type Integer))
  (`self.TurnActor`))

(event `self.Box.OnComponentBeginOverlap`
  (params (OverlappedComponent :type "PrimitiveComponent Object Reference") (OtherActor :type "Actor Object Reference") (OtherComp :type "PrimitiveComponent Object Reference") (OtherBodyIndex :type Integer) (bFromSweep :type Boolean) (SweepResult :type "HitResult Structure (by ref)"))
  (`self.TurnActor`))

(event `PlayDead`
  (set `self.b_Dead` true)
  (`PaperFlipbookComponent.SetFlipbook` (`self.Sprite`) "/Game/Assets/Tiles/Characters/slimeDead_Flipbook.slimeDead_Flipbook")
  (`GameplayStatics.PlaySound2D` "/Game/Audio/enemyHit.enemyHit" 1.0 1.0 0.0 null null)
  (`KismetSystemLibrary.Delay` 0.2)
  (`self.K2_DestroyActor`))

(fn `UserConstructionScript`)