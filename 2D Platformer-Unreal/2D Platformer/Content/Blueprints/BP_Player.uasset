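; Player character for a 2D side-scrolling platformer, starting paused, with movement, jumping, flipbook animation and velocity-based facing.
; A box overlap kills slimes, while capsule contact costs health and triggers blinking immunity, with health and score stored in PS_2DGame.
; BeginPlay builds parallax dynamic materials on background sprites, and Tick offsets the spring arm to hold camera height.
; The downward-trace stomp check, CheckHit, is left unused.
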(event `CheckHit`
  (bind _returnvalue (`SceneComponent.K2_GetComponentLocation` (`self.Scene`)))
  ;[1 1 1] Raycasting to check whther the player is landing on enemy or not
  (if (`NavMovementComponent.IsFalling` (`self.CharacterMovement`))
    (`|ExecutionSequence`
      (:`then_0`
        (bind _outhit (`KismetSystemLibrary.LineTraceSingle` :`Start` _returnvalue :`End` (+ _returnvalue (* (0.0 0.0 -1.0) (`self.f_TraceLength`))) :`TraceChannel` "TraceTypeQuery1" :`DrawDebugType` "ForDuration"))
        (bind _asbp_slime (cast `/Game/Blueprints/BP_Slime` (`.HitActor` (`GameplayStatics.BreakHitResult` _outhit))))
        (`/Game/Blueprints/BP_Slime.PlayDead` _asbp_slime)
        (`KismetSystemLibrary.PrintString` "slime at bottom")))))

(event `self.ReceiveBeginPlay`
  (set `PlayerController.bShowMouseCursor` true (`GameplayStatics.GetPlayerController` 0))
  (set `self.b_Pause` true)
  ;[1 1 1] creating parallax effect
  (for (_array_element _array_index) (`SceneComponent.GetChildrenComponents` (`self.PaperSprite6`) false)
    (bind _aspaper_sprite_component (cast `PaperSpriteComponent` _array_element))
    (bind _returnvalue (`PrimitiveComponent.CreateDynamicMaterialInstance` _aspaper_sprite_component 0 null "None"))
    (`KismetArrayLibrary.Array_Add` (`self.DynamicLayers`) _returnvalue)
    (`MaterialInstanceDynamic.SetScalarParameterValue` _returnvalue "ParallaxMultiplier" (`|GetArrayItem` (`self.F_ParallaxMultiplier`) _array_index))))

(event `self.ReceiveTick`
  (params (DeltaSeconds :type "Float (single-precision)"))
  (bind (_returnvalue_x _returnvalue_y _returnvalue_z) (`KismetMathLibrary.BreakVector` (`SceneComponent.K2_GetComponentLocation` (`self.CapsuleComponent`))))
  (if (not (`self.b_Pause`))
    (`self.HandleAnimation`)
    (`self.HandleRotation`)
    ;[1 1 1] Camera offset to keep y-pos constant
    (set `SpringArmComponent.TargetOffset` (`KismetMathLibrary.MakeVector` 0.0 0.0 (- (`self.F_CamerHeight`) _returnvalue_z)) (`self.SpringArm`))
    ;[1 1 1] Blinking effect to make player look immune
    (if (`self.b_Immune`)
      (`PaperFlipbookComponent.SetSpriteColor` (`self.Sprite`) (struct :`R` 1.0 :`G` 1.0 :`B` 1.0))
      (`KismetSystemLibrary.Delay` 0.1)
      (`PaperFlipbookComponent.SetSpriteColor` (`self.Sprite`) (struct :`R` 1.0 :`G` 1.0 :`B` 1.0 :`A` 1.0))
      (`KismetSystemLibrary.Delay` 1.0)
      (`PaperFlipbookComponent.SetSpriteColor` (`self.Sprite`) (struct :`R` 1.0 :`G` 1.0 :`B` 1.0 :`A` 1.0))
      (set `self.b_Immune` false))))

(event `InputAction|Jump`
  (params (Key :type "Key Structure"))
  (:`Pressed`
    (if (`self.b_Pause`)
      _
      (elif (`NavMovementComponent.IsMovingOnGround` (`self.CharacterMovement`))
        (`self.Jump`)
        (`GameplayStatics.PlaySound2D` "/Game/Audio/jump.jump" 1.0 1.0 0.0 null null))))
  (:`Released`
    (if (not (`self.b_Pause`))
      (`self.StopJumping`))))

(event `InputAxis|Horizontal`
  (params (AxisValue :type "Float (single-precision)"))
  (if (not (`self.b_Pause`))
    (if (> AxisValue 0.0)
      (set `self.isMovinfRight?` true)
      (elif (< AxisValue 0.0)
        (set `self.isMovinfRight?` false)))
    (`self.AddMovementInput` (1.0 0.0 0.0) AxisValue)))

(event `HandleAnimation`
  (if (`NavMovementComponent.IsFalling` (`self.CharacterMovement`))
    (`PaperFlipbookComponent.SetFlipbook` (`self.Sprite`) "/Game/Assets/Tiles/Characters/Jump.Jump")
    (else
      ;[1 1 1] Handeling idle and movement animations
      (if (> (`KismetMathLibrary.VSize` (`MovementComponent.Velocity` (`self.CharacterMovement`))) 0.0)
        (`PaperFlipbookComponent.SetFlipbook` (`self.Sprite`) "/Game/Assets/Tiles/Characters/Move.Move")
        (else
          (`PaperFlipbookComponent.SetFlipbook` (`self.Sprite`) "/Game/Assets/Tiles/Characters/Idle.Idle"))))))

(event `HandleRotation`
  (bind _velocity_x (`KismetMathLibrary.BreakVector` (`MovementComponent.Velocity` (`self.CharacterMovement`))))
  ;[1 1 1] Changing rotations according to the player velocity.
  (`/Engine/EditorBlueprintResources/StandardMacros.IsValid` (`self.GetController`)
    (:`Is Valid`
      (`/Engine/EditorBlueprintResources/StandardMacros.CompareFloat` _velocity_x
        (:`>`
          (`Controller.SetControlRotation` (`self.GetController`) (`KismetMathLibrary.MakeRotator` 0.0 0.0 180.0) :!label _label))
        (:`==`
          (if (`self.isMovinfRight?`)
            (goto _label)
            (else
              (`Controller.SetControlRotation` (`self.GetController`) (`KismetMathLibrary.MakeRotator` 0.0) :!label _label_2))))
        (:`<`
          (goto _label_2))))))

(event `GiveScore`
  (params (ScoreCount :type Integer))
  (bind _asps_2dgame (cast `/Game/Blueprints/PS_2DGame` (`self.PlayerState`)))
  (set `/Game/Blueprints/PS_2DGame.i_Score` (+ (`/Game/Blueprints/PS_2DGame.i_Score` _asps_2dgame) ScoreCount) _asps_2dgame))

(event `self.CapsuleComponent.OnComponentBeginOverlap`
  (params (OverlappedComponent :type "PrimitiveComponent Object Reference") (OtherActor :type "Actor Object Reference") (OtherComp :type "PrimitiveComponent Object Reference") (OtherBodyIndex :type Integer) (bFromSweep :type Boolean) (SweepResult :type "HitResult Structure (by ref)"))
  (bind _asbp_slime (cast `/Game/Blueprints/BP_Slime` OtherActor))
  (if (`/Game/Blueprints/BP_Slime.b_Dead` _asbp_slime)
    _
    (elif (not (`self.b_Immune`))
      (bind _asps_2dgame (cast `/Game/Blueprints/PS_2DGame` (`self.PlayerState`)))
      (bind _result (`/Engine/EditorBlueprintResources/StandardMacros.DecrementInt` (`/Game/Blueprints/PS_2DGame.i_Health` _asps_2dgame))
        (:`  `
          (`KismetSystemLibrary.PrintString` "slime collided")
          (`GameplayStatics.PlaySound2D` "/Game/Audio/heroHit.heroHit" 1.0 1.0 0.0 null null)
          (set `self.b_Immune` true)
          (if (== _result 0)
            (`GameplayStatics.OpenLevelBySoftObjectPtr` "/Game/Level/2DGameNew.2DGameNew")
            (bind _aspc_main (cast `/Game/Blueprints/PC_Main` (`self.GetController`)))
            (set `PlayerController.bShowMouseCursor` true _aspc_main)))))))

(event `AddHealth`
  (bind _asps_2dgame (cast `/Game/Blueprints/PS_2DGame` (`self.PlayerState`)))
  (`/Engine/EditorBlueprintResources/StandardMacros.IncrementInt` (`/Game/Blueprints/PS_2DGame.i_Health` _asps_2dgame)))

(event `self.Box.OnComponentBeginOverlap`
  (params (OverlappedComponent :type "PrimitiveComponent Object Reference") (OtherActor :type "Actor Object Reference") (OtherComp :type "PrimitiveComponent Object Reference") (OtherBodyIndex :type Integer) (bFromSweep :type Boolean) (SweepResult :type "HitResult Structure (by ref)"))
  (bind _asbp_slime (cast `/Game/Blueprints/BP_Slime` OtherActor))
  (`/Game/Blueprints/BP_Slime.PlayDead` _asbp_slime))

(fn `UserConstructionScript`)